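; Player controller for a mouse-driven camera that pans, orbits and zooms around the point under the cursor.
; A visibility trace, or a fixed point along the cursor ray on a miss, sets the pivot, marked by a spawned BP_Focus actor.
; Left drag pans on the pivot's horizontal plane, right drag orbits it within pitch and height limits.
; The wheel lerps the pawn toward or away from it with a swept move.
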(event Custom|SetPOI
  (params (POILocation :type Vector))
  ;[1 1 1] POI
  (Transformation|SetWorldLocation (Variables|/Script/Engine.Actor|GetRootComponent (Variables|Default|GetBP_Focus)) POILocation false false))

(event Custom|TurnUP
  (params (B :type Float%20%28single-precision%29))
  (bind _returnvalue (Transformation|GetActorRightVector))
  (bind _returnvalue_2 (* -3.0 B))
  (bind _self self)
  (bind _pitchmin (Variables|Default|GetPitchMin))
  (bind _pitchmax (Variables|Default|GetPitchMax))
  (bind _returnvalue_3 (Pawn|GetControlRotation _self :!class /Script/Engine.Controller))
  (bind _returnvalue_4 (Math|Vector|RotatorfromAxisandAngle _returnvalue _returnvalue_2))
  (bind _returnvalue_5 (Math|Rotator|CombineRotators _returnvalue_3 _returnvalue_4))
  (bind (_roll _pitch _yaw) (Math|Rotator|BreakRotator _returnvalue_5))
  ;[1 1 1] 上下旋转
  (if (Variables|Default|GetbRightDown)
    (Development|PrintString "上下旋转" false)
    (bind _output_get (Variables|Default|SetPawnLocationInitial (Transformation|GetActorLocation (Pawn|GetControlledPawn))))
    (if (Math|Boolean|ANDBoolean (<= (.Z (Math|Vector|BreakVector (+ (Variables|Default|GetClickLocation) (Math|Vector|RotateVectorAroundAxis (- _output_get (Variables|Default|GetClickLocation)) _returnvalue_2 _returnvalue)))) (Variables|Default|GetHighMax)) (>= _pitch _pitchmin) (<= _pitch _pitchmax))
      (Pawn|SetControlRotation self (Math|Rotator|MakeRotator 0.0 (Math|Float|Clamp(Float) _pitch _pitchmin _pitchmax) _yaw))
      (Transformation|SetActorLocation (Pawn|GetControlledPawn) (+ (Variables|Default|GetClickLocation) (Math|Vector|RotateVectorAroundAxis (- _output_get (Variables|Default|GetClickLocation)) _returnvalue_2 _returnvalue)) false false))))

(event Custom|TurnRight
  (params (NewParam :type Float%20%28single-precision%29))
  (bind _returnvalue (Math|Vector|MakeVector 0.0 0.0 1.0))
  (bind _returnvalue_2 (* 3.0 NewParam))
  (bind _self self)
  ;[1 1 1] 左右旋转
  (if (Variables|Default|GetbRightDown)
    (Development|PrintString "左右旋转" false)
    (bind _output_get (Variables|Default|SetPawnLocationInitial (Transformation|GetActorLocation (Pawn|GetControlledPawn))))
    (Transformation|SetActorLocation (Pawn|GetControlledPawn) (+ (Variables|Default|GetClickLocation) (Math|Vector|RotateVectorAroundAxis (- _output_get (Variables|Default|GetClickLocation)) _returnvalue_2 _returnvalue)) false false)
    (Pawn|SetControlRotation _self (Math|Rotator|CombineRotators (Pawn|GetControlRotation _self :!class /Script/Engine.Controller) (Math|Vector|RotatorfromAxisandAngle _returnvalue _returnvalue_2)))))

(event Custom|ShowPOI
  (params (bShow :type Boolean))
  ;[1 1 1] POI
  (Rendering|SetVisibility (Variables|/Script/Engine.Actor|GetRootComponent (Variables|Default|GetBP_Focus)) bShow false))

(event Custom|Handle%20pan%20movement
  (bind (_worldlocation _worlddirection) (Game|Player|ConvertMouseLocationToWorldSpace))
  ;[0.05 0.05 0.05] 平移计算
  (if (Variables|Default|GetbLeftDown)
    (Transformation|AddActorWorldOffset (Pawn|GetControlledPawn) (* (- (Variables|Default|GetLast%20mouse%20trace%20location) (Utilities|GetMouseandHorizontalPlaneHitLocation _worldlocation _worlddirection (Variables|Default|GetLast%20mouse%20trace%20location))) 1.0))))

(event EventTick
  (params (DeltaSeconds :type Float%20%28single-precision%29))
  ;[1 1 1] Tick
  (Utilities|FlowControl|Sequence
    (:then_0
      (if (Math|Boolean|ORBoolean (Variables|Default|GetbRightDown) (Variables|Default|GetbLeftDown) (Variables|Default|GetbWheeling))
        (CallFunction|ShowPOI true)
        (else
          (CallFunction|ShowPOI false))))))

(event EventBeginPlay
  ;[1 1 1] Begin
  (Utilities|FlowControl|Sequence
    (:then_0
      (bind _returnvalue (Game|SpawnActorfromClass "/Game/MouseControl1/BP_Focus.BP_Focus_C" (Math|Transform|MakeTransform "0, 0, 0") "Undefined" self 0))
      (Variables|Default|SetBP_Focus _returnvalue))
    (:then_1
      (Variables|Default|SetPawnLocationTarget (Transformation|GetActorLocation (Pawn|GetControlledPawn)))
      (Variables|Default|SetPawnRotationTarget (Pawn|GetControlRotation self :!class /Script/Engine.Controller)))))

(event Input|MouseEvents|MouseY
  (params (AxisValue :type Float%20%28single-precision%29))
  ;[0.000407 0.03 0] 鼠标按键
  (if (!= AxisValue 0.0)
    (Utilities|FlowControl|Sequence
      (:then_0
        (CallFunction|TurnUP AxisValue))
      (:then_1
        (CallFunction|HandlePanMovement)))))

(event Input|MouseEvents|MouseX
  (params (AxisValue :type Float%20%28single-precision%29))
  ;[0.000407 0.03 0] 鼠标按键
  (if (!= AxisValue 0.0)
    (Utilities|FlowControl|Sequence
      (:then_0
        (CallFunction|TurnRight AxisValue))
      (:then_1
        (CallFunction|HandlePanMovement)))))

(event Input|MouseEvents|MouseWheelUp
  (params (Key :type Key%20Structure :default "None"))
  (bind _returnvalue (CallFunction|GetZhongXinPoint))
  (bind _zoomspeed (Variables|Default|GetZoomSpeed))
  ;[1 1 1] 滚轮缩放
  (:Pressed
    (if (not (or (Variables|Default|GetbLeftDown) (Variables|Default|GetbRightDown)))
      ;;[1 1 1] 1~4
      (Development|PrintString "放大" false)
      (Variables|Default|SetbWheeling true)
      (bind (_hit _distance _location) (CallFunction|MouseHit))
      (if _hit
        (CallFunction|SetPOI _location)
        (CallFunction|CameraZoom true _distance _zoomspeed _location)
        (else
          (CallFunction|SetPOI _returnvalue)
          (CallFunction|CameraZoom true 1e+01 _zoomspeed _returnvalue)))
      (Utilities|FlowControl|RetriggerableDelay 0.2)
      (Variables|Default|SetbWheeling false))))

(event Input|MouseEvents|MouseWheelDown
  (params (Key :type Key%20Structure :default "None"))
  (bind _returnvalue (CallFunction|GetZhongXinPoint))
  ;[1 1 1] 滚轮缩放
  (:Pressed
    (if (not (or (Variables|Default|GetbLeftDown) (Variables|Default|GetbRightDown)))
      ;;[1 1 1] -1~-4
      (Development|PrintString "缩小" false)
      (Variables|Default|SetbWheeling true)
      (bind (_hit _distance _location) (CallFunction|MouseHit))
      (if _hit
        (CallFunction|SetPOI _location)
        (CallFunction|CameraZoom true _distance 0.0 _location)
        (else
          (CallFunction|SetPOI _returnvalue)
          (CallFunction|CameraZoom true 1e+01 0.0 _returnvalue)))
      (Utilities|FlowControl|RetriggerableDelay 0.2)
      (Variables|Default|SetbWheeling false))))

(event Input|MouseEvents|LeftMouseButton
  (params (Key :type Key%20Structure :default "None"))
  ;[1 1 1] 鼠标左键移动视角
  (:Pressed
    (if (not (Variables|Default|GetbRightDown))
      (Variables|Default|SetbLeftDown true)
      (bind (_hit _distance _location) (CallFunction|MouseHit))
      (if _hit
        (bind _output_get (Variables|Default|SetLast%20mouse%20trace%20location _location))
        (CallFunction|SetPOI _output_get)
        (else
          (bind _output_get_2 (Variables|Default|SetLast%20mouse%20trace%20location (CallFunction|GetZhongXinPoint)))
          (CallFunction|SetPOI _output_get_2)))))
  (:Released
    (Variables|Default|SetbLeftDown false)))

(event Input|MouseEvents|RightMouseButton
  (params (Key :type Key%20Structure :default "None"))
  ;[1 1 1] 右键按下旋转视角
  (:Pressed
    (if (not (Variables|Default|GetbLeftDown))
      (Variables|Default|SetbRightDown true)
      (bind (_hit _distance _location) (CallFunction|MouseHit))
      (if _hit
        (if (>= _distance 1e+01)
          (Variables|Default|SetClickLocation _location)
          (CallFunction|SetPOI (Variables|Default|GetClickLocation) :!label _label))
        (else
          (Variables|Default|SetClickLocation (CallFunction|GetZhongXinPoint))
          (goto _label)))))
  (:Released
    (Variables|Default|SetbRightDown false)))

(fn ConstructionScript)

(fn MouseHit
  (bind _self self)
  (bind (_worldlocation _worlddirection) (Game|Player|ConvertMouseLocationToWorldSpace _self))
  (bind (_outhit _returnvalue) (Collision|LineTraceByChannel _worldlocation (+ _worldlocation (* _worlddirection 2147483647)) "TraceTypeQuery1" true 0 "None" true "(R=1.000000,G=0.000000,B=0.000000,A=1.000000)" "(R=0.000000,G=1.000000,B=0.000000,A=1.000000)" 1e+02))
  (if _returnvalue
    (Development|PrintString (Utilities|String|Append "点击到物体：" (Utilities|GetDisplayName (.HitActor (Collision|BreakHitResult _outhit))) "物体的距离：" (Utilities|String|ToString(Float) (.Distance (Collision|BreakHitResult _outhit)))) false)
    (return true (.Distance (Collision|BreakHitResult _outhit)) (.Location (Collision|BreakHitResult _outhit)))
    (else
      (Development|PrintString "没有点击到物体" false)
      (return false 0.0 "0, 0, 0"))))

(fn CameraZoom
  (params (Hit :type Boolean) (Diatance :type Float%20%28single-precision%29) (Clamp :type Float%20%28single-precision%29) (Location :type Vector))
  (bind _returnvalue (Pawn|GetControlledPawn))
  (bind _returnvalue_2 (Class|Actor|GetInputAxisKeyValue))
  (bind _zoomspeed (Variables|Default|GetZoomSpeed))
  (bind _returnvalue_3 (/ 1e+02 _zoomspeed))
  (bind _returnvalue_4 (Transformation|GetActorLocation _returnvalue))
  (bind _returnvalue_5 (/ _returnvalue_2 _returnvalue_3))
  (bind _returnvalue_6 (Math|Vector|Lerp(Vector) _returnvalue_4 Location _returnvalue_5))
  (if Hit
    (if (>= Diatance Clamp)
      (Development|PrintString (Utilities|String|Append "Pawn:" (Utilities|String|ToString(Vector) _returnvalue_4) "Hit:" (Utilities|String|ToString(Vector) Location) "New:" (Utilities|String|ToString(Vector) _returnvalue_6) "Distance:" (Utilities|String|ToString(Float) (Math|Vector|VectorLength (- _returnvalue_4 Location)))) false)
      (if (<= (.Z (Math|Vector|BreakVector _returnvalue_6)) (Variables|Default|GetHighMax))
        (bind _returnvalue_7 (Transformation|SetActorLocation (Pawn|GetControlledPawn) _returnvalue_6 true false))
        (Development|PrintString (Utilities|String|ToString(Boolean) _returnvalue_7) false)))))

(fn GetZhongXinPoint
  (bind _self self)
  (bind (_worldlocation _worlddirection) (Game|Player|ConvertMouseLocationToWorldSpace _self))
  (return (+ _worldlocation (* _worlddirection 2000))))